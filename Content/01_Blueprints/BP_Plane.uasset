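; Player plane Blueprint that sets up Enhanced Input and the main HUD, with boost, missile fire and quit actions.
; Boost multiplies BPEngineComponent's speed force for a set duration while Tick eases the spring arm to a boost length and back.
; Holding fire runs a looping timer spawning BP_Missile at both spawners.
; Stop-engine cuts Niagara exhaust and reapplies current velocity, but its speed-force zeroing is unconnected; release restores both defaults.
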(event Input|EnhancedActionEvents|EnhancedInputActionIA_Boost
  (params (ActionValue :type Boolean) (ElapsedSeconds :type Float%20%28double-precision%29) (TriggeredSeconds :type Float%20%28double-precision%29) (InputAction :type Input%20Action%20Object%20Reference :default "/Game/05_Inputs/IA_Boost.IA_Boost"))
  (bind _bp_enginecomponent (Variables|Default|GetBP_EngineComponent))
  (bind _bp_enginecomponent_2 (Variables|Default|GetBP_EngineComponent))
  (:Started
    (if (and (Math|Float|NearlyEqual(Float) (Variables|/Script/Engine.SpringArmComponent|GetTargetArmLength (Variables|Default|GetSpringArm)) (Variables|Default|GetDefaultCamArmLength) 1e+02) (not (Variables|Default|GetIsBoosting)))
      (Development|PrintString "Boost")
      (Variables|Default|SetIsBoosting true)
      (Variables|/Game/01_Blueprints/Components/BP_EngineComponent.BP_EngineComponent_C|SetCurrentSpeedForce _bp_enginecomponent (* (Variables|/Game/01_Blueprints/Components/BP_EngineComponent.BP_EngineComponent_C|GetBaseSpeedForce _bp_enginecomponent) (Variables|/Game/01_Blueprints/Components/BP_EngineComponent.BP_EngineComponent_C|GetMultiplyBoostSpeedForce _bp_enginecomponent)))
      (Utilities|FlowControl|Delay (Variables|Default|GetBoostDuration))
      (Variables|Default|SetIsBoosting false)
      (Variables|/Game/01_Blueprints/Components/BP_EngineComponent.BP_EngineComponent_C|SetCurrentSpeedForce _bp_enginecomponent_2 (Variables|/Game/01_Blueprints/Components/BP_EngineComponent.BP_EngineComponent_C|GetBaseSpeedForce _bp_enginecomponent_2)))))

(event Input|EnhancedActionEvents|EnhancedInputActionIA_Exit
  (params (ActionValue :type Boolean) (ElapsedSeconds :type Float%20%28double-precision%29) (TriggeredSeconds :type Float%20%28double-precision%29) (InputAction :type Input%20Action%20Object%20Reference :default "/Game/05_Inputs/IA_Exit.IA_Exit"))
  (:Triggered
    (Development|PrintString "Hello" :!label _label)
    (Game|QuitGame 0 "Quit" false))
  (:Started
    (goto _label)))

(event Input|EnhancedActionEvents|EnhancedInputActionIA_StopEngine
  (params (ActionValue :type Boolean) (ElapsedSeconds :type Float%20%28double-precision%29) (TriggeredSeconds :type Float%20%28double-precision%29) (InputAction :type Input%20Action%20Object%20Reference :default "/Game/05_Inputs/IA_StopEngine.IA_StopEngine"))
  (bind _staticmesh (Variables|Default|GetStaticMesh))
  (bind _bp_enginecomponent (Variables|Default|GetBP_EngineComponent))
  (:Triggered
    (Physics|SetPhysicsLinearVelocity _staticmesh (Transformation|GetComponentVelocity _staticmesh) false "None")
    (CallFunction|SetEngineNiagaraSpawnRate 0.0))
  (:Completed
    (Variables|/Game/01_Blueprints/Components/BP_EngineComponent.BP_EngineComponent_C|SetCurrentSpeedForce _bp_enginecomponent (Variables|/Game/01_Blueprints/Components/BP_EngineComponent.BP_EngineComponent_C|GetBaseSpeedForce _bp_enginecomponent))
    (CallFunction|SetEngineNiagaraSpawnRate (Variables|Default|GetNiagaraDefaultSpeed))))

(event Input|EnhancedActionEvents|EnhancedInputActionIA_ShootMissile
  (params (ActionValue :type Boolean) (ElapsedSeconds :type Float%20%28double-precision%29) (TriggeredSeconds :type Float%20%28double-precision%29) (InputAction :type Input%20Action%20Object%20Reference :default "/Game/05_Inputs/IA_ShootMissile.IA_ShootMissile"))
  (:Started
    (bind _returnvalue (Utilities|Time|SetTimerbyFunctionName 0 "SpawnAllMissiles" (Variables|Default|GetMissileInterval) true true))
    (Variables|Default|SetTimerMissileSpawner _returnvalue))
  (:Canceled
    (Utilities|Time|ClearandInvalidateTimerbyHandle (Variables|Default|GetTimerMissileSpawner) :!label _label))
  (:Completed
    (goto _label)))

(event EventBeginPlay
  (bind _returnvalue (Game|GetPlayerController 0))
  (bind _returnvalue_2 (PlayerController|LocalPlayerSubsystems|GetEnhancedInputLocalPlayerSubsystem _returnvalue))
  (Utilities|IsValid _returnvalue_2
    (:Is%20Valid
      (Input|AddMappingContext _returnvalue_2 "/Game/05_Inputs/IMC_Plane.IMC_Plane" 0 "(bIgnoreAllPressedKeysUntilRelease=True,bForceImmediately=False,bNotifyUserSettings=False)")
      (Variables|Default|SetMissileSpawners (Utilities|Array|MakeArray (Variables|Default|GetML) (Variables|Default|GetMR)))
      (Variables|Default|SetDefaultCamArmLength (Variables|/Script/Engine.SpringArmComponent|GetTargetArmLength (Variables|Default|GetSpringArm)))
      (bind _returnvalue_3 (UserInterface|CreateWidget "/Game/01_Blueprints/Widgets/WB_MainWidget.WB_MainWidget_C"))
      (bind _output_get (Variables|Default|SetMainWidget _returnvalue_3))
      (UserInterface|Viewport|AddtoViewport _output_get 0)
      (CallFunction|SetEngineNiagaraSpawnRate (Variables|Default|GetNiagaraDefaultSpeed))
      (Variables|/Script/Engine.PlayerController|SetbShowMouseCursor (Game|GetPlayerController 0) true))))

(event EventTick
  (params (DeltaSeconds :type Float%20%28single-precision%29))
  (bind _isboosting (Variables|Default|GetIsBoosting))
  (bind _springarm (Variables|Default|GetSpringArm))
  (if (or (!= (Variables|/Script/Engine.SpringArmComponent|GetTargetArmLength (Variables|Default|GetSpringArm)) (Variables|Default|GetDefaultCamArmLength)) _isboosting)
    (if _isboosting
      (Variables|/Script/Engine.SpringArmComponent|SetTargetArmLength _springarm (Math|Interpolation|FInterpTo (Variables|/Script/Engine.SpringArmComponent|GetTargetArmLength _springarm) (+ (Variables|Default|GetBoostCamArmLength) (Variables|Default|GetDefaultCamArmLength)) (Utilities|Time|GetWorldDeltaSeconds) 3.5))
      (else
        (Variables|/Script/Engine.SpringArmComponent|SetTargetArmLength _springarm (Math|Interpolation|FInterpTo (Variables|/Script/Engine.SpringArmComponent|GetTargetArmLength _springarm) (Variables|Default|GetDefaultCamArmLength) (Utilities|Time|GetWorldDeltaSeconds) 1.0))))))

(event Collision|EventActorBeginOverlap
  (params (OtherActor :type Actor%20Object%20Reference))
  (Development|PrintString "AAAAAAAHHH"))

(fn ConstructionScript)

(fn SpawnMissile
  (params (SpawnLocation :type Scene%20Component%20Object%20Reference))
  (Game|SpawnActorfromClass "/Game/01_Blueprints/BP_Missile.BP_Missile_C" (Transformation|GetWorldTransform SpawnLocation) "AdjustIfPossibleButAlwaysSpawn" "MultiplyWithRoot" 0 0))

(fn SpawnAllMissiles
  (bind _array_element (Utilities|Array|ForEachLoopwithBreak (Variables|Default|GetMissileSpawners))
    (:LoopBody
      (CallFunction|SpawnMissile _array_element))))

(fn SetEngineNiagaraSpawnRate
  (params (NewSpawnRate :type Float%20%28double-precision%29))
  (Effects|Components|ParticleSystem|SetFloatParameter (Variables|Default|GetNiagara) "User.SpawnRate" NewSpawnRate))