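; Engine component that drives its owner's physics-simulating root primitive, treated as a plane, along its right vector as forward.
; BeginPlay keeps the root only if it simulates physics and seeds the base speed.
; While the engine is on, Tick ramps speed by acceleration up to a cap, then overwrites linear velocity with that forward speed plus the negated off-axis velocity.
; Mouse-aimed force steering and debug nodes remain disconnected.
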(event EventBeginPlay
  (bind _asprimitive_component (Utilities|Casting|CastToPrimitiveComponent (Variables|/Script/Engine.Actor|GetRootComponent (Components|GetOwner))))
  (bind _output_get (Variables|Default|SetRefToPlane _asprimitive_component))
  (if (Physics|IsSimulatingPhysics _output_get "None")
    (Variables|Default|SetCurrentSpeedForce (Variables|Default|GetBaseSpeed))
    (else
      (Variables|Default|SetRefToPlane 0))))

(event EventTick
  (params (DeltaSeconds :type Float%20%28single-precision%29))
  (bind _reftoplane (Variables|Default|GetRefToPlane))
  (bind _returnvalue (Math|Vector|GetRightVector _reftoplane))
  (bind _returnvalue_2 (Transformation|GetComponentVelocity _reftoplane))
  (Variables|Default|GetRefToPlane
    (:then
      (if (Variables|Default|GetIsEngineOn)
        (Variables|Default|SetCurrentSpeedForce (Math|Float|Clamp(Float) (+ (Variables|Default|GetCurrentSpeedForce) (* (Variables|Default|GetAcceleration) (Utilities|Time|GetWorldDeltaSeconds))) 0.0 (Variables|Default|GetMaxSpeedForce)))
        (Physics|SetPhysicsLinearVelocity _reftoplane (+ (* (Variables|Default|GetCurrentSpeedForce) _returnvalue) (* (- _returnvalue_2 (* _returnvalue (Math|Vector|DotProduct _returnvalue _returnvalue_2))) -1.0)) false "None")))
    (:else)))