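; BP_ScoreManager tracks the plane player's score and a countdown, ending the game on a win or timeout.
; After the plane's start delay, it counts BP_Point actors as the target score and starts a looping one-second, pausable timer.
; UpdateScore increments the score; reaching the target or running out of time shows WB_EndScreen, freezes global time dilation and pauses engine audio.
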(event EventBeginPlay
  (bind _asbp_plane (Utilities|Casting|CastToBP_Plane (Game|Player|GetPlayerPawn 0)))
  (Utilities|FlowControl|Delay (Variables|/Game/01_Blueprints/BP_Plane.BP_Plane_C|GetDelayBegining _asbp_plane))
  (bind _outactors (Actor|GetAllActorsOfClass "/Game/01_Blueprints/BP_Point.BP_Point_C"))
  (Variables|Default|SetScoreMax (Utilities|Array|Length _outactors))
  (Variables|Default|SetPlayerScore 0)
  (Variables|Default|SetTimer (Variables|Default|GetMaxTimer))
  (bind _returnvalue (Utilities|Time|SetTimerbyFunctionName 0 "TimerFunction" 1.0 true true 1.0))
  (Variables|Default|SetFonctionHandler _returnvalue))

(fn TimerFunction
  (bind _timer (Variables|Default|GetTimer))
  (if (not (Variables|Default|GetTimerPaused))
    (Math|Float|DecrementFloat _timer
      (:%20%20
        (if (<= _timer 0.0)
          (Variables|Default|SetTextEnd "Time's up")
          (CallFunction|TheEndFunction))))))

(fn UpdateScore
  (bind _playerscore (Variables|Default|GetPlayerScore))
  (Math|Integer|IncrementInt _playerscore
    (:%20%20
      (if (>= _playerscore (Variables|Default|GetScoreMax))
        (Variables|Default|SetTextEnd "Congrats!")
        (CallFunction|TheEndFunction)))))

(fn TheEndFunction
  (bind _returnvalue (UserInterface|CreateWidget "/Game/01_Blueprints/Widgets/WB_EndScreen.WB_EndScreen_C"))
  (bind _output_get (Variables|Default|SetEndWidget _returnvalue))
  (UserInterface|Viewport|AddtoViewport _output_get 0)
  (Utilities|Time|SetGlobalTimeDilation 0.0)
  (bind _asbp_plane (Utilities|Casting|CastToBP_Plane (Game|Player|GetPlayerPawn 0)))
  (Class|AudioComponent|SetPaused (Variables|/Game/01_Blueprints/BP_Plane.BP_Plane_C|GetEngineAudio _asbp_plane) true))