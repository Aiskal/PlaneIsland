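; Actor component that rotates its owner's root primitive, referenced as a plane, to follow the mouse cursor.
; BeginPlay caches the root; each Tick normalizes the cursor's offset from viewport center and scales it by the max rotation limits.
; Vertical offset sets roll, while horizontal offset sets pitch and is added to current yaw, so off-center input keeps turning.
; RInterpTo smooths the result at RotationSpeed, applied as a teleporting world rotation without sweep.
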(event EventBeginPlay
  (bind _asprimitive_component (Utilities|Casting|CastToPrimitiveComponent (Variables|/Script/Engine.Actor|GetRootComponent (Components|GetOwner))))
  (Variables|Default|SetRef%20to%20Plane _asprimitive_component))

(event EventTick
  (params (DeltaSeconds :type Float%20%28single-precision%29))
  (bind _returnvalue (Game|GetPlayerController 0))
  (bind _returnvalue_2 (Viewport|GetViewportSize))
  (bind _ref_to_plane (Variables|Default|GetRef%20to%20Plane))
  (bind _max_rotation_tb (Variables|Default|GetMax%20Rotation%20TB))
  (bind _ref_to_plane_2 (Variables|Default|GetRef%20to%20Plane))
  (bind _max_rotation_lr (Variables|Default|GetMax%20Rotation%20LR))
  (bind (_locationx _locationy) (Game|Player|GetMousePosition _returnvalue))
  (bind _returnvalue_3 (Transformation|GetWorldRotation _ref_to_plane))
  (bind _returnvalue_4 (/ _returnvalue_2 2.0))
  (bind _returnvalue_5 (- _locationx (.x _returnvalue_4)))
  (bind _returnvalue_6 (- _locationy (.y _returnvalue_4)))
  (bind _returnvalue_7 (/ _returnvalue_5 (.x _returnvalue_4)))
  (bind _returnvalue_8 (/ _returnvalue_6 (.y _returnvalue_4)))
  (bind _returnvalue_9 (* _returnvalue_7 _max_rotation_lr))
  (bind _returnvalue_10 (* _returnvalue_8 _max_rotation_tb))
  (bind _returnvalue_11 (Math|Rotator|MakeRotator _returnvalue_10 _returnvalue_9 _returnvalue_9))
  (Variables|Default|GetRef%20to%20Plane
    (:then
      (Transformation|SetWorldRotation _ref_to_plane_2 (Math|Interpolation|RInterpTo (Transformation|GetWorldRotation _ref_to_plane_2) (Math|Rotator|MakeRotator (+ (- (.roll _returnvalue_11) (.roll _returnvalue_3)) (.roll _returnvalue_3)) (.pitch _returnvalue_11) (+ (.yaw _returnvalue_11) (.yaw _returnvalue_3))) (Utilities|Time|GetWorldDeltaSeconds) (Variables|Default|GetRotation%20Speed)) false true))
    (:else)))