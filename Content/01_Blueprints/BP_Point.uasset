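; BP_Point is a score target that breaks when the player's BP_Plane or a BP_Missile overlaps its sphere.
; Each such overlap spawns and triggers an FS_MasterField field system at the point's location and passes its Infos to the plane cached after BeginPlay.
; The first scored hit also plays audio, updates the plane's score manager, clears IsNotShot and destroys the actor after a configurable delay.
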(event OnComponentBeginOverlap(Sphere)
  (params (OverlappedComponent :type Primitive%20Component%20Object%20Reference) (OtherActor :type Actor%20Object%20Reference) (OtherComp :type Primitive%20Component%20Object%20Reference) (OtherBodyIndex :type Integer) (bFromSweep :type Boolean) (SweepResult :type Hit%20Result%20Structure%20%28by%20ref%29))
  (Utilities|Casting|CastToBP_Plane OtherActor
    (:then
      _)
    (:CastFailed
      (Utilities|Casting|CastToBP_Missile OtherActor)))
  (bind _returnvalue (Game|SpawnActorfromClass "/Engine/EditorResources/FieldNodes/FS_MasterField.FS_MasterField_C" (Math|Transform|MakeTransform (.location (Transformation|GetActorTransform)) "0, 0, 0" "3.000000,3.000000,3.000000") "Undefined" "MultiplyWithRoot" 0 0))
  (Variables|/Engine/EditorResources/FieldNodes/FS_MasterField.FS_MasterField_C|SetActivationType _returnvalue "NewEnumerator4")
  (Default|CETrigger _returnvalue)
  (bind _planepawn (Variables|Default|GetPlanePawn)
    (:then
      (Variables|/Game/01_Blueprints/BP_Plane.BP_Plane_C|SetLastInfo _planepawn (Variables|Default|GetInfos))
      (if (Variables|Default|GetIsNotShot)
        (bind _returnvalue_2 (AddComponent|AddAudioComponent false))
        (Audio|Components|Audio|SetVolumeMultiplier _returnvalue_2 (Variables|Default|GetVolumeMultiply) :!class /Script/Engine.AudioComponent)
        (Default|UpdateScore (Variables|/Game/01_Blueprints/BP_Plane.BP_Plane_C|GetBP_ScoreManager _planepawn))
        (Variables|Default|SetIsNotShot false)
        (Utilities|FlowControl|Delay (Variables|Default|GetLifeSpanBeforeDepop) :!label _label)
        (Actor|DestroyActor)))
    (:else
      (goto _label))))

(event EventBeginPlay
  (Utilities|FlowControl|Delay 2.0)
  (bind _asbp_plane (Utilities|Casting|CastToBP_Plane (Game|Player|GetPlayerPawn 0)))
  (Variables|Default|SetPlanePawn _asbp_plane))

(fn ConstructionScript)